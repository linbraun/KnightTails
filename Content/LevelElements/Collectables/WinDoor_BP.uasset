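; Exit door for the cat knight side-scroller that loads the win map once the player has collected enough keys.
; Overlapping its trigger box enables Interact input and shows both prompt and error widgets.
; Interact checks the key count through the game mode, then plays a portal sound and opens the level.
; Leaving the box calls DisableInput and hides both widgets after a short delay.
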(event OnComponentBeginOverlap(TriggerBox)
  (params (OverlappedComponent :type Primitive%20Component%20Object%20Reference) (OtherActor :type Actor%20Object%20Reference) (OtherComp :type Primitive%20Component%20Object%20Reference) (OtherBodyIndex :type Integer) (bFromSweep :type Boolean) (SweepResult :type Hit%20Result%20Structure%20%28by%20ref%29))
  (Utilities|Casting|CastToSideScrollerCharacter_CatKnight OtherActor)
  (Input|EnableInput (Game|GetPlayerController 0))
  (Development|SetHiddeninGame (Variables|Default|GetPromptWidget) false false))

(event OnComponentEndOverlap(TriggerBox)
  (params (OverlappedComponent :type Primitive%20Component%20Object%20Reference) (OtherActor :type Actor%20Object%20Reference) (OtherComp :type Primitive%20Component%20Object%20Reference) (OtherBodyIndex :type Integer))
  (Utilities|Casting|CastToSideScrollerCharacter_CatKnight OtherActor)
  (Input|DisableInput (Game|GetPlayerController 0) 0)
  (Utilities|FlowControl|Delay 0.9)
  (Development|SetHiddeninGame 0 true false))

(event Input|ActionEvents|InputActionInteract
  (params (Key :type Key%20Structure :default "None"))
  ;[1 1 1] Win Condition
  (:Pressed
    (bind _gamemode (Class|GameModeINT|GetGameModeRef(Message) (Game|GetGameMode)))
    (if (>= (Variables|/Game/LevelBlueprints/CatKnightRunner_GM.CatKnightRunner_GM_C|GetKeys _gamemode) 3)
      (Audio|PlaySoundatLocation "/Game/Recycle/SuperGrid/TutorialLevel/SoundEffects/Cue_Portals.Cue_Portals" "0, 0, 0" "0, 0, 0" 1.0 1.0 0.0 0 0 0)
      (Game|OpenLevel(byName) "Win_Map"))))

(fn ConstructionScript)