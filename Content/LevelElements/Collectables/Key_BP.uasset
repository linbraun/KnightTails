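; Collectable key for the CatKnight side-scroller, picked up by pressing Interact while the player is nearby.
; A timeline animates the key's height from BeginPlay, while the trigger sphere toggles actor input and the prompt widget for Player-tagged actors.
; A one-time interact posts a key message through the game mode, calls KeyAmount on the game instance and plays a sound.
; A loot timeline then animates the actor before destroying it.
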(event OnComponentEndOverlap(TriggerSphere)
  (params (OverlappedComponent :type Primitive%20Component%20Object%20Reference) (OtherActor :type Actor%20Object%20Reference) (OtherComp :type Primitive%20Component%20Object%20Reference) (OtherBodyIndex :type Integer))
  ;[1 1 1] Enable/Disable Input
  (if (Actor|ActorHasTag OtherActor "Player")
    (Input|DisableInput (Game|GetPlayerController 0))
    ;[1 1 1] Display Interact Prompt
    (Utilities|FlowControl|Delay 0.9)
    (Development|SetHiddeninGame 0 true false)))

(event OnComponentBeginOverlap(TriggerSphere)
  (params (OverlappedComponent :type Primitive%20Component%20Object%20Reference) (OtherActor :type Actor%20Object%20Reference) (OtherComp :type Primitive%20Component%20Object%20Reference) (OtherBodyIndex :type Integer) (bFromSweep :type Boolean) (SweepResult :type Hit%20Result%20Structure%20%28by%20ref%29))
  ;[1 1 1] Enable/Disable Input
  (if (Actor|ActorHasTag OtherActor "Player")
    (Input|EnableInput (Game|GetPlayerController 0))
    ;[1 1 1] Display Interact Prompt
    (Development|SetHiddeninGame (Variables|Default|GetInteractWidget) false false)))

(event Custom|KeyLooted
  (bind _returnvalue (Transformation|GetActorLocation))
  (bind _returnvalue_2 (Transformation|GetActorRotation))
  (Rendering|SetVisibility (Variables|Default|GetKey_P) false false)
  (bind (_direction _locationalpha _rotationalpha) (Timeline|KeyLootMovement Play)
    (:Update
      (Transformation|SetActorRelativeLocation (Math|Vector|MakeVector (.x _returnvalue) (.y _returnvalue) (+ (.z _returnvalue) (.Z (Math|Vector|BreakVector _locationalpha)))))
      (Transformation|SetActorRelativeLocation (Math|Vector|MakeVector (.roll _returnvalue_2) (.pitch _returnvalue_2) _rotationalpha)))
    (:Finished
      (Actor|DestroyActor))))

(event EventBeginPlay
  (bind _locationalpha (Timeline|StartMovement Play)
    (:Update
      (Transformation|SetRelativeLocation (Variables|Default|GetKey) (Math|Vector|MakeVector 0.0 0.0 (.Z (Math|Vector|BreakVector _locationalpha))) false false))))

(event Input|ActionEvents|InputActionInteract
  (params (Key :type Key%20Structure :default "None"))
  (:Pressed
    (Utilities|FlowControl|DoOnce false
      (:Completed
        (Utilities|Casting|CastToSideScrollerCharacter_CatKnight (Game|GetPlayerCharacter 0))
        (bind _gamemode (Class|GameModeINT|GetGameModeRef(Message) (Game|GetGameMode)))
        (Class|GameModeINT|AddKey(Message) _gamemode)
        (bind _ascat_knight_runner_gi (Utilities|Casting|CastToCatKnightRunner_GI (Game|GetGameInstance)))
        (Default|KeyAmount _ascat_knight_runner_gi)
        (Audio|PlaySoundatLocation 0 "0, 0, 0" "0, 0, 0" 1.0 1.0 0.0 0 0 0)
        (CallFunction|KeyLooted)))))

(fn ConstructionScript)