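; Falling spike trap that shakes, drops and damages what it hits when an actor tagged Player enters its trigger box.
; The first overlap plays a Movement timeline that rolls the Arrow component as a wobble, then after a delay stops it and enables physics on the spike.
; The first hit on the spike applies obstacle damage once.
; Shortly after the drop, the actor destroys itself and spawns a steam effect at the spike's location.
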(event OnComponentBeginOverlap(Box)
  (params (OverlappedComponent :type Primitive%20Component%20Object%20Reference) (OtherActor :type Actor%20Object%20Reference) (OtherComp :type Primitive%20Component%20Object%20Reference) (OtherBodyIndex :type Integer) (bFromSweep :type Boolean) (SweepResult :type Hit%20Result%20Structure%20%28by%20ref%29))
  ;[1 1 1] Activate Falling Spike
  (if (Actor|ActorHasTag OtherActor "Player")
    (if (not (Variables|Default|GetFallingSpikeTriggered))
      (bind _floatmovement (Timeline|Movement Play)
        (:Update
          (Transformation|SetWorldRotation (Variables|Default|GetArrow) (Math|Rotator|Lerp(Rotator) "0, 0, 0" (Math|Rotator|MakeRotator 5.0 0.0 0.0) _floatmovement) false false)
          (Variables|Default|SetFallingSpikeTriggered true)
          (Utilities|FlowControl|Delay 2.0)
          (Utilities|FlowControl|Sequence
            (:then_0
              (Timeline|Movement Stop))
            (:then_1
              (Physics|SetSimulatePhysics (Variables|Default|GetFallingSpike) true)
              (Utilities|FlowControl|Delay 2.0)
              (bind _output_get (Variables|Default|SetSpikeLocation (Transformation|GetWorldLocation (Variables|Default|GetFallingSpike))))
              (Actor|DestroyActor)
              (Effects|SpawnEmitteratLocation "/Game/LevelDesign/StarterContent/Particles/P_Steam_Lit.P_Steam_Lit" _output_get))))))))

(event OnComponentHit(FallingSpike)
  (params (HitComponent :type Primitive%20Component%20Object%20Reference) (OtherActor :type Actor%20Object%20Reference) (OtherComp :type Primitive%20Component%20Object%20Reference) (NormalImpulse :type Vector :default "0, 0, 0") (Hit :type Hit%20Result%20Structure%20%28by%20ref%29))
  ;[1 1 1] On Hit
  (if (not (Variables|Default|GetFallingSpikeHit))
    (Game|Damage|ApplyDamage OtherActor (Variables|Default|GetObstacle%20Damage) 0 0)
    (Variables|Default|SetFallingSpikeHit true)))

(event EventBeginPlay
  ;[1 1 1] Begin Play
  (Variables|Default|SetSpikeLocation (Transformation|GetActorLocation))
  (Variables|Default|SetSpikeRotation (Transformation|GetWorldRotation (Variables|Default|GetArrow))))

(fn ConstructionScript)