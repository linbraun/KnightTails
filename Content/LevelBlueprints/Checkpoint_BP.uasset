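; Checkpoint actor for CatKnight Runner that sets the player's respawn point when touched.
; On overlap with player 0, it writes its SpawnTransform to the CatKnightRunner_GM game mode, converting the location to world space while keeping rotation as stored and scale at one.
; The construction script moves the Capsule to SpawnTransform to show that point.
; Game-mode message, dust, sound and test logic are disconnected and never run.
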(event OnComponentBeginOverlap(Box)
  (params (OverlappedComponent :type Primitive%20Component%20Object%20Reference) (OtherActor :type Actor%20Object%20Reference) (OtherComp :type Primitive%20Component%20Object%20Reference) (OtherBodyIndex :type Integer) (bFromSweep :type Boolean) (SweepResult :type Hit%20Result%20Structure%20%28by%20ref%29))
  ;[1 1 1] Spawn Location & Sound
)

(event Collision|EventActorBeginOverlap
  (params (OtherActor :type Actor%20Object%20Reference))
  ;[1 1 1] Spawn Transform
  (if (== OtherActor (Game|GetPlayerCharacter 0))
    (bind _ascat_knight_runner_gm (Utilities|Casting|CastToCatKnightRunner_GM (Game|GetGameMode)))
    (Variables|/Game/LevelBlueprints/CatKnightRunner_GM.CatKnightRunner_GM_C|SetSpawnTransform _ascat_knight_runner_gm (Math|Transform|MakeTransform (Math|Transform|TransformLocation (Transformation|GetActorTransform) (.location (Variables|Default|GetSpawnTransform))) (.rotation (Variables|Default|GetSpawnTransform)) "1,1,1"))))

(fn ConstructionScript
  (Transformation|SetRelativeTransform (Variables|Default|GetCapsule) (Variables|Default|GetSpawnTransform) false false))