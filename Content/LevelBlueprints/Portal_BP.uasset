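; Portal actor that moves the player's Cat Knight to a named checkpoint when the player enters it.
; A trigger box overlap by an actor tagged Player looks up the portal's Name in the game mode's Checkpoint map.
; Game mode and Cat Knight references come through message getters, and player pawn 0's root is set to that location without sweep or teleport physics.
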(event OnComponentBeginOverlap(TriggerBox)
  (params (OverlappedComponent :type Primitive%20Component%20Object%20Reference) (OtherActor :type Actor%20Object%20Reference) (OtherComp :type Primitive%20Component%20Object%20Reference) (OtherBodyIndex :type Integer) (bFromSweep :type Boolean) (SweepResult :type Hit%20Result%20Structure%20%28by%20ref%29))
  (if (Actor|ActorHasTag OtherActor "Player")
    (bind _gamemode (Class|GameModeINT|GetGameModeRef(Message) (Game|GetGameMode)))
    (bind _catknight (Class|CatKnightINT|GetCatKnightRef(Message) (Game|Player|GetPlayerPawn 0)))
    (bind _catknight_2 (Class|CatKnightINT|GetCatKnightRef(Message) _catknight))
    (Transformation|SetWorldLocation (Variables|/Script/Engine.Actor|GetRootComponent _catknight_2) (.Value (Utilities|Map|Find (Variables|/Game/LevelBlueprints/CatKnightRunner_GM.CatKnightRunner_GM_C|GetCheckpoint _gamemode) (Variables|Default|GetName))) false false)))

(event EventBeginPlay)

(event Collision|EventActorBeginOverlap
  (params (OtherActor :type Actor%20Object%20Reference)))

(event EventTick
  (params (DeltaSeconds :type Float%20%28single-precision%29)))

(fn ConstructionScript)